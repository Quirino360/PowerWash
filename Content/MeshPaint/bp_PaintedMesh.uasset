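; Skeletal mesh actor that supports runtime painting at a given position and normal, using a render-target mask cleared on BeginPlay.
; UnWrap temporarily swaps slot 0 to M_Unwrap, scene-captures only that mesh, then restores its materials.
; Paint runs UnWrap, feeds position and normal into a new M_PaintTexture instance, and draws it into CRT_PaintMask.
; Each paint call also draws a debug arrow along the normal.
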(event EventBeginPlay
  (Rendering|ClearRenderTarget2D "/Game/MeshPaint/CRT_PaintMask.CRT_PaintMask"))

(fn ConstructionScript)

(fn UnWrap
  (bind _scenecapturecomponent2d (Variables|Default|GetSceneCaptureComponent2D))
  (bind _skeletalmesh (Variables|Default|GetSkeletalMesh))
  (Transformation|SetWorldRotation _scenecapturecomponent2d "-90.000000,-90.000000,0.000000" false false)
  (Rendering|SceneCapture|ShowOnlyComponent _scenecapturecomponent2d _skeletalmesh)
  (Variables|Default|SetTMP_Materials (Rendering|Material|GetMaterials _skeletalmesh))
  (Rendering|Material|SetMaterial _skeletalmesh 0 "/Game/MeshPaint/m_Unwrap.m_Unwrap")
  (Rendering|SceneCapture|CaptureScene (Variables|Default|GetSceneCaptureComponent2D) :!class /Script/Engine.SceneCaptureComponent2D)
  (for (_array_element _array_index) (Variables|Default|GetTMP_Materials)
    (Rendering|Material|SetMaterial (Variables|Default|GetSkeletalMesh) _array_index _array_element)))

(fn Paint
  (params (Position :type Vector) (Normal :type Vector))
  (Rendering|Debug|DrawDebugArrow Position (+ Position (* Normal 5e+01)) 1.0 "(R=0.000000,G=0.993799,B=1.000000,A=1.000000)" 1.0 1.0)
  (CallFunction|UnWrap)
  (bind _returnvalue (Rendering|Material|CreateDynamicMaterialInstance "/Game/MeshPaint/m_PaintTexture.m_PaintTexture" "None" "None" :!class /Script/Engine.KismetMaterialLibrary))
  (Rendering|Material|SetVectorParameterValue _returnvalue "Position" (Math|Conversions|ToLinearColor(Vector) Position) :!class /Script/Engine.MaterialInstanceDynamic)
  (Rendering|Material|SetVectorParameterValue _returnvalue "Normal" (Math|Conversions|ToLinearColor(Vector) Normal) :!class /Script/Engine.MaterialInstanceDynamic)
  (Rendering|DrawMaterialtoRenderTarget "/Game/MeshPaint/CRT_PaintMask.CRT_PaintMask" _returnvalue))